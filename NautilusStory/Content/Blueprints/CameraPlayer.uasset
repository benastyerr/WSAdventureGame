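; CameraPlayer is a camera Blueprint that can register itself as the player's starting camera.
; On BeginPlay it checks the "save" slot; if no save exists, or the saved Camera is invalid, an instance flagged IsFirstCamera passes itself to the Player through SetNewCamera and SetNewCam.
; When the save holds a valid Camera, it does nothing.
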(event `self.ReceiveBeginPlay`
  (bind _returnvalue (`GameplayStatics.DoesSaveGameExist` "save"))
  (if _returnvalue
    (bind _returnvalue_2 (`GameplayStatics.LoadGameFromSlot` "save"))
    (bind _assave (cast `/Game/Player/Save` _returnvalue_2))
    (`/Game/Player/Save.camera` _assave
      (:`then`)
      (:`else`
        _)))
  (if (`self.isFirstCamera`)
    (bind _asplayer (cast `/Game/Player/Player` (`GameplayStatics.GetPlayerCharacter` 0)))
    (`/Game/Player/Player.SetNewCamera` _asplayer self)
    (`/Game/Player/Player.SetNewCam` _asplayer self)))

(fn `UserConstructionScript`)