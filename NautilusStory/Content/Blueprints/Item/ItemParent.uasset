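; Parent Blueprint for pickup items, each described by an ItemStructure and shown with a Cylinder component.
; Get adds the icon to the Player's Inventory, stores the structure in the CustomGameInstance Items list, then destroys the actor.
; SetMaterial swaps the cylinder's first material.
; Combine only destroys this actor when the target is another ItemParent, with no result item created here.
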(event `/Game/Blueprints/Item/ObjectInterface.Get`
  (bind (_itemstructure_name _itemstructure_description _itemstructure_model3d _itemstructure_icon) (break `/Game/Blueprints/Item/ItemStructure` (`self.itemStructure`)))
  (bind _asplayer (cast `/Game/Player/Player` (`GameplayStatics.GetPlayerCharacter` 0)))
  (`/Game/Widgets/W_Inventory.AddObject` (`/Game/Player/Player.Inventory` _asplayer) _itemstructure_icon)
  (bind _ascustom_game_instance (cast `/Game/Player/CustomGameInstance` (`GameplayStatics.GetGameInstance`)))
  (`KismetArrayLibrary.Array_Add` (`/Game/Player/CustomGameInstance.items` _ascustom_game_instance) (`self.itemStructure`))
  (`self.K2_DestroyActor`))

(event `/Game/Blueprints/Item/ObjectInterface.SetMaterial`
  (params (materialToSet :type "Material Object Reference"))
  (`PrimitiveComponent.SetMaterial` (`self.Cylinder`) 0 materialToSet))

(event `/Game/Blueprints/Item/ObjectInterface.Combine`
  (params (actorToUseWith :type "Actor Object Reference"))
  (cast `/Game/Blueprints/Item/ItemParent` actorToUseWith)
  (`self.K2_DestroyActor`))

(fn `UserConstructionScript`)