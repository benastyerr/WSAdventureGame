(event `self.ReceiveBeginPlay`
  (bind (_itemstructure_name _itemstructure_description _itemstructure_class _itemstructure_icon) (break `/Game/Blueprints/Items/Parent/ItemsStructure` (`self.itemStructure`)))
  (set `self.itemStructure` (make `/Game/Blueprints/Items/Parent/ItemsStructure` _itemstructure_name _itemstructure_description _itemstructure_class _itemstructure_icon self)))

(event `/Game/Blueprints/Items/Parent/ObjectInterface.Get`
  (bind _itemstructure_name (break `/Game/Blueprints/Items/Parent/ItemsStructure` (`self.itemStructure`)))
  (bind (_itemstructure_name_2 _itemstructure_description _itemstructure_class _itemstructure_icon) (break `/Game/Blueprints/Items/Parent/ItemsStructure` (`self.itemStructure`)))
  (bind _asplayer (cast `/Game/Player/Player` (`GameplayStatics.GetPlayerCharacter` 0)))
  (`/Game/Widgets/W_Inventory.AddObject` (`/Game/Player/Player.Inventory` _asplayer) _itemstructure_icon)
  (bind _ascustom_game_instance (cast `/Game/Player/CustomGameInstance` (`GameplayStatics.GetGameInstance`)))
  (`KismetArrayLibrary.Array_Add` (`/Game/Player/CustomGameInstance.items` _ascustom_game_instance) (`self.itemStructure`))
  (`/Game/Widgets/W_PopUp.Make Notification` (`/Game/Player/Player.W Pop Up` _asplayer) (`|FormatText` "You found a <Bold> {item} </>" _itemstructure_name) true 3.0)
  (bind _asplayer_2 (cast `/Game/Player/Player` (`GameplayStatics.GetPlayerCharacter` 0)))
  (`/Game/Player/LevelSave.AddToArray` (`/Game/Player/PointAndClickGamemode.LevelSaveObject` (`/Game/Player/Player.Gamemode` _asplayer_2)) self)
  (`self.K2_DestroyActor`))

(fn `UserConstructionScript`
  (`parent.UserConstructionScript`))