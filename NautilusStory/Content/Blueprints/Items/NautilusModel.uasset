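; Nautilus model item that opens a 3D inspection menu when picked and serves as a combine target for unlocking a linked door.
; Selecting its Cube while combining a NautilusPiece runs Combine, which, if CanOpenDoor is set, closes the menu, unlocks and messages the door once, records itself for saving and destroys the Cube.
; A successful combine consumes the inventory piece.
; Activation clears CanOpenDoor, so combining then just closes the menu.
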(event `self.Get`
  (bind (_returnvalue_location _returnvalue_rotation _returnvalue_scale) (`KismetMathLibrary.BreakTransform` (`self.GetTransform`)))
  (bind (_itemstructure_name _itemstructure_description _itemstructure_class) (break `/Game/Blueprints/Items/Parent/ItemStructure` (`self.itemStructure`)))
  (bind _asplayer (cast `/Game/Player/Player` (`GameplayStatics.GetPlayerCharacter` 0)))
  (`/Game/Player/Player.Open3DMenu` _asplayer _itemstructure_class (`KismetMathLibrary.MakeTransform` _returnvalue_location (struct :`Yaw` 90.0) _returnvalue_scale) (`self.Door`) true null "Visible"))

(event `/Game/Blueprints/Items/3DinteractionInterface.SetVar`
  (params (actorToSet :type "Actor Object Reference"))
  (set `self.Door` actorToSet))

(event `self.Activation`
  (set `self.canOpenDoor` false))

(event `/Game/Blueprints/Items/3DinteractionInterface.Select`
  (params (actor :type "ActorComponent Object Reference"))
  (if (== actor (`self.Cube`))
    (bind _asplayer (cast `/Game/Player/Player` (`GameplayStatics.GetPlayerCharacter` 0)))
    (if (`/Game/Player/Player.isCombining` _asplayer)
      (bind _objectdestroyed (`self.Combine` (`/Game/Player/Player.selectedObject` _asplayer)))
      (if _objectdestroyed
        (bind _asplayer_2 (cast `/Game/Player/Player` (`GameplayStatics.GetPlayerCharacter` 0)))
        (bind _ascustom_game_instance (cast `/Game/Player/CustomGameInstance` (`GameplayStatics.GetGameInstance`)))
        (bind _inventory (`/Game/Player/Player.Inventory` _asplayer_2))
        (bind _selectedindex (`/Game/Widgets/W_Inventory.selectedIndex` _inventory))
        (`KismetArrayLibrary.Array_Remove` (`/Game/Player/CustomGameInstance.items` _ascustom_game_instance) _selectedindex)
        (`/Game/Widgets/W_Inventory.RemoveObject` _inventory _selectedindex)
        (`/Game/Widgets/W_Inventory.Unselect` _inventory)))))

(fn `Combine`
  (params (actorToUseWith :type "Actor Object Reference"))
  (returns (objectDestroyed :type Boolean))
  (cast `/Game/Blueprints/Items/NautilusPiece` actorToUseWith
    (:`then`
      (if (`self.canOpenDoor`)
        (`/Engine/EditorBlueprintResources/StandardMacros.DoOnce` false
          (:`Completed`
            (bind _asplayer (cast `/Game/Player/Player` (`GameplayStatics.GetPlayerCharacter` 0)))
            (`/Game/Player/Player.Close3DMenu` _asplayer)
            (bind _door (`self.Door`)
              (:`then`
                (bind _asmoving_door (cast `/Game/Blueprints/Doors/MovingDoor` _door)
                  (:`then`
                    (set `/Game/Blueprints/Doors/MovingDoor.isLocked` false _asmoving_door))
                  (:`CastFailed`
                    _))
                (message `/Game/Blueprints/Items/Parent/ObjectInterface.Get` _door)
                (`/Game/Player/LevelSave.AddToArray` (`/Game/Player/PointAndClickGamemode.LevelSaveObject` (`/Game/Player/Player.Gamemode` _asplayer)) self)
                (bind _cube (`self.Cube`)
                  (:`then`
                    (`ActorComponent.K2_DestroyComponent` _cube))
                  (:`else`
                    _))
                (return true))
              (:`else`))))
        (else
          (bind _asplayer_2 (cast `/Game/Player/Player` (`GameplayStatics.GetPlayerCharacter` 0)))
          (`/Game/Player/Player.Close3DMenu` _asplayer_2)
          (return false))))
    (:`CastFailed`
      (return false))))

(fn `UserConstructionScript`
  (`parent.UserConstructionScript`))