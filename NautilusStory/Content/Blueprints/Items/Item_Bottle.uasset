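; Bottle item actor that the player collects through its Get event.
; Get adds the item's icon to the player's Inventory and appends its ItemStructure to the Items collection on the custom game instance.
; It then shows a W_Notification widget with the item's name and icon and destroys the actor.
; The construction script only calls its parent.
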(event `/Game/Blueprints/Items/Parent/ObjectInterface.Get`
  (bind (_itemstructure_name _itemstructure_description _itemstructure_class _itemstructure_icon) (break `/Game/Blueprints/Items/Parent/ItemStructure` (`self.itemStructure`)))
  (bind (_itemstructure_name_2 _itemstructure_description_2 _itemstructure_class_2 _itemstructure_icon_2) (break `/Game/Blueprints/Items/Parent/ItemStructure` (`self.itemStructure`)))
  (bind _asplayer (cast `/Game/Player/Player` (`GameplayStatics.GetPlayerCharacter` 0)))
  (`/Game/Widgets/W_Inventory.AddObject` (`/Game/Player/Player.Inventory` _asplayer) _itemstructure_icon_2)
  (bind _ascustom_game_instance (cast `/Game/Player/CustomGameInstance` (`GameplayStatics.GetGameInstance`)))
  (`KismetArrayLibrary.Array_Add` (`/Game/Player/CustomGameInstance.items` _ascustom_game_instance) (`self.itemStructure`))
  (bind _returnvalue (`|CreateWidget` "/Game/Widgets/W_Notification.W_Notification_C"))
  (`UserWidget.AddToViewport` _returnvalue 0)
  (`/Game/Widgets/W_Notification.Make Notification` _returnvalue _itemstructure_name "" _itemstructure_icon)
  (`self.K2_DestroyActor`))

(fn `UserConstructionScript`
  (`parent.UserConstructionScript`))