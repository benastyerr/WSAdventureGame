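; LevelOpener is a trigger box that moves the player to another level when their capsule overlaps it.
; It freezes player movement, shows a transition widget with the destination name, and opens the target level after a delay.
; If a save named after the current level exists, it first stores the player's transform there as the last location.
; A short delay after BeginPlay arms the trigger, so earlier overlaps are ignored.
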(event `self.Box.OnComponentBeginOverlap`
  (params (OverlappedComponent :type "PrimitiveComponent Object Reference") (OtherActor :type "Actor Object Reference") (OtherComp :type "PrimitiveComponent Object Reference") (OtherBodyIndex :type Integer) (bFromSweep :type Boolean) (SweepResult :type "HitResult Structure (by ref)"))
  (bind _asplayer (cast `/Game/Player/Player` OtherActor))
  (if (`self.canTP`)
    (if (== OtherComp (`Character.CapsuleComponent` _asplayer))
      (set `/Game/Player/Player.canMove` false _asplayer)
      (bind _returnvalue (`|CreateWidget` "/Game/Widgets/W_Transition.W_Transition_C" null true (`self.LevelName`)))
      (`UserWidget.AddToViewport` _returnvalue 0)
      (bind _returnvalue_2 (`GameplayStatics.GetCurrentLevelName` true))
      (bind _returnvalue_3 (`GameplayStatics.DoesSaveGameExist` _returnvalue_2))
      (if _returnvalue_3
        (bind _returnvalue_4 (`GameplayStatics.GetCurrentLevelName` true))
        (bind _returnvalue_5 (`GameplayStatics.LoadGameFromSlot` _returnvalue_4))
        (bind _aslevel_save (cast `/Game/Player/LevelSave` _returnvalue_5))
        (set `/Game/Player/LevelSave.lastplayerlocation` (`self.GetTransform` (`GameplayStatics.GetPlayerCharacter` 0)) _aslevel_save)
        (`GameplayStatics.SaveGameToSlot` _returnvalue_5 _returnvalue_4))
      (`KismetSystemLibrary.Delay` 2.0)
      (`GameplayStatics.OpenLevelBySoftObjectPtr` (`self.levelToOpen`)))))

(event `self.ReceiveBeginPlay`
  (`KismetSystemLibrary.Delay` 0.2)
  (set `self.canTP` true))

(fn `UserConstructionScript`)