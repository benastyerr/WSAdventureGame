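; Guard is an actor that switches to a punching state when the Player enters its box trigger.
; On BeginPlay it passes a reference to itself to its AB_Guard animation instance.
; The box overlap sets the Punching flag and snaps the guard's rotation to the look-at direction from the player toward the guard.
; Nothing in this Blueprint clears the flag.
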(event `self.ReceiveBeginPlay`
  (bind _asab_guard (cast `/Game/Blueprints/Guard/AB_Guard` (`SkeletalMeshComponent.GetAnimInstance` (`self.SkeletalMesh`))))
  (set `/Game/Blueprints/Guard/AB_Guard.guardRef` self _asab_guard))

(event `self.Box.OnComponentBeginOverlap`
  (params (OverlappedComponent :type "PrimitiveComponent Object Reference") (OtherActor :type "Actor Object Reference") (OtherComp :type "PrimitiveComponent Object Reference") (OtherBodyIndex :type Integer) (bFromSweep :type Boolean) (SweepResult :type "HitResult Structure (by ref)"))
  (bind _asplayer (cast `/Game/Player/Player` OtherActor))
  (set `self.punching` true)
  (`self.K2_SetActorRotation` (`KismetMathLibrary.FindLookAtRotation` (`self.K2_GetActorLocation` _asplayer) (`self.K2_GetActorLocation`))))

(fn `UserConstructionScript`)