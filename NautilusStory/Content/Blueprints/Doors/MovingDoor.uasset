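; A door actor that registers an objective with the custom game instance on BeginPlay and can be raised vertically.
; Get, if the door is unlocked, plays a one-shot opening sound and timeline lerp, then adds the door to the level save object.
; Activation instead jumps the door straight to its raised position, sets IsLocked and removes the objective.
; Combine always returns false.
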(event `self.ReceiveBeginPlay`
  (set `self.firstLocation` (`self.K2_GetActorLocation`))
  (bind _ascustom_game_instance (cast `/Game/Player/CustomGameInstance` (`GameplayStatics.GetGameInstance`)))
  (`/Game/Player/CustomGameInstance.AddObjective` _ascustom_game_instance (`self.ObjectiveName`) (`self.ObjectiveDescription`)))

(event `/Game/Blueprints/Items/Parent/ObjectInterface.Activation`
  (set `self.isLocked` true)
  (`self.K2_SetActorLocation` (+ (`self.firstLocation`) (0.0 0.0 400.0)) true)
  (bind _ascustom_game_instance (cast `/Game/Player/CustomGameInstance` (`GameplayStatics.GetGameInstance`)))
  (`/Game/Player/CustomGameInstance.RemoveObjective` _ascustom_game_instance (`self.ObjectiveName`)))

(event `/Game/Blueprints/Items/Parent/ObjectInterface.Get`
  (bind _firstlocation (`self.firstLocation`))
  (if (not (`self.isLocked`))
    (`/Engine/EditorBlueprintResources/StandardMacros.DoOnce` (`self.isLocked`)
      (:`Completed`
        (`GameplayStatics.SpawnSound2D` "/Game/Sound/SFX/GateOpen.GateOpen" 1.0 1.0 0.0 null)
        (bind (_direction _newtrack_0) (`Timeline|MoveDoorTimeline` :!via `PlayFromStart`)
          (:`Update`
            (`self.K2_SetActorLocation` (`KismetMathLibrary.VLerp` _firstlocation (+ _firstlocation (0.0 0.0 400.0)) _newtrack_0) true))
          (:`Finished`
            (bind _asplayer (cast `/Game/Player/Player` (`GameplayStatics.GetPlayerCharacter` 0)))
            (`/Game/Player/LevelSave.AddToArray` (`/Game/Player/PointAndClickGamemode.LevelSaveObject` (`/Game/Player/Player.Gamemode` _asplayer)) self)
            (set `self.isLocked` false)))))))

(fn `Combine`
  (params (actorToUseWith :type "Actor Object Reference"))
  (returns (objectDestroyed :type Boolean))
  (return false))

(fn `UserConstructionScript`)