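; Interactable cabin door that can be locked, highlighted and swung open, optionally registering an objective with the game instance.
; While locked, SetMaterial toggles a highlight made from a duplicate mesh.
; Combine unlocks it with any actor, as the lockpick cast is unwired; Get then plays a timeline rotation and saves the door to level data.
; Activation snaps it open, re-locks it and clears the objective.
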(event `self.ReceiveBeginPlay`
  (set `self.firstRot` (`SceneComponent.K2_GetComponentRotation` (`self.SceneRef`)))
  (if (`self.objectif`)
    (bind _ascustom_game_instance (cast `/Game/Player/CustomGameInstance` (`GameplayStatics.GetGameInstance`)))
    (`/Game/Player/CustomGameInstance.AddObjective` _ascustom_game_instance (`self.ObjectiveName`) (`self.ObjectiveDescription`))))

(event `self.SetMaterial`
  (params (canSetOutline :type Boolean))
  (bind _door (`self.Door`))
  (if (`self.isLocked`)
    (if (`self.isOpen`)
      (bind _outlinemesh (`self.outlineMesh` :!label _label)
        (:`then`
          (`ActorComponent.K2_DestroyComponent` _outlinemesh)
          (goto _label_2 :!via `Reset`))
        (:`else`))
      (elif canSetOutline
        (`/Engine/EditorBlueprintResources/StandardMacros.DoOnce` false :!label _label_2
          (:`Completed`
            (bind _returnvalue (`AddComponent|NODE_AddStaticMeshComponent-0` :`RelativeTransform` (`SceneComponent.GetRelativeTransform` _door)))
            (bind _output_get (set `self.outlineMesh` _returnvalue))
            (`StaticMeshComponent.SetStaticMesh` _output_get (`StaticMeshComponent.StaticMesh` _door))
            (for _ (range (`KismetArrayLibrary.Array_Length` (`MeshComponent.GetMaterials` (`self.outlineMesh`))))
              (`PrimitiveComponent.SetMaterial` (`self.outlineMesh`) 0 "/Game/Blueprints/Items/Parent/Inst_ItemHighLight.Inst_ItemHighLight"))))
        (else
          (goto _label))))))

(event `self.Get`
  (bind (_firstrot_roll _firstrot_pitch _firstrot_yaw) (`KismetMathLibrary.BreakRotator` (`self.firstRot`)))
  (if (not (`self.isLocked`))
    (`/Engine/EditorBlueprintResources/StandardMacros.DoOnce` false
      (:`Completed`
        (bind _asplayer (cast `/Game/Player/Player` (`GameplayStatics.GetPlayerCharacter` 0)))
        (set `self.isOpen` true)
        (bind _selectableobject (`/Game/Player/Player.selectableObject` _asplayer))
        (`KismetArrayLibrary.Array_Remove` _selectableobject (`KismetArrayLibrary.Array_Find` _selectableobject self))
        (`self.SetMaterial` false)
        (`GameplayStatics.SpawnSound2D` "/Game/Sound/SFX/Porte.Porte" 1.0 1.0 0.0 null)
        (`|ExecutionSequence`
          (:`then_0`
            (bind (_direction _alpha) (`Timeline|Timeline` :!via `PlayFromStart`)
              (:`Update`
                (`SceneComponent.K2_SetWorldRotation` (`self.SceneRef`) (`KismetMathLibrary.RLerp` (`self.firstRot`) (`KismetMathLibrary.MakeRotator` _firstrot_roll _firstrot_pitch (+ _firstrot_yaw (`self.rotationRef`))) _alpha) false false))
              (:`Finished`
                (set `self.isOpen` true)
                (bind _outlinemesh (`self.outlineMesh`)
                  (:`then`
                    (`ActorComponent.K2_DestroyComponent` _outlinemesh))
                  (:`else`)))))
          (:`then_1`
            (bind _asplayer_2 (cast `/Game/Player/Player` (`GameplayStatics.GetPlayerCharacter` 0)))
            (bind _gamemode (`/Game/Player/Player.Gamemode` _asplayer_2))
            (`/Game/Player/LevelSave.AddToArray` (`/Game/Player/PointAndClickGamemode.LevelSaveObject` _gamemode) self)
            (`/Game/Player/PointAndClickGamemode.SaveLevelData` _gamemode)))))))

(event `self.Activation`
  (bind (_firstrot_roll _firstrot_pitch _firstrot_yaw) (`KismetMathLibrary.BreakRotator` (`self.firstRot`)))
  (set `self.isLocked` true)
  (set `self.isOpen` true)
  (`SceneComponent.K2_SetWorldRotation` (`self.SceneRef`) (`KismetMathLibrary.MakeRotator` _firstrot_roll _firstrot_pitch (+ _firstrot_yaw (`self.rotationRef`))) false false)
  (bind _ascustom_game_instance (cast `/Game/Player/CustomGameInstance` (`GameplayStatics.GetGameInstance`)))
  (`/Game/Player/CustomGameInstance.RemoveObjective` _ascustom_game_instance (`self.ObjectiveName`)))

(fn `Combine`
  (params (actorToUseWith :type "Actor Object Reference"))
  (returns (objectDestroyed :type Boolean))
  (set `self.isLocked` false)
  (`GameplayStatics.SpawnSound2D` "/Game/Sound/Vis.Vis" 1.0 1.0 0.0 null)
  (return true))

(fn `UserConstructionScript`)