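; PNJ is an interactable NPC that opens a dialogue with the player and can be outlined as a highlight.
; Get creates the dialogue widget, starts the AI controller's dialogue with the GameInstance's tree or its own as fallback, then locks player movement.
; SetMaterial spawns a copy of the Cube mesh with a highlight material, guarded by a DoOnce, and destroys it when turned off.
; Combine always returns false.
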(event `/Game/Blueprints/Items/Parent/ObjectInterface.Get`
  (bind _returnvalue (`|CreateWidget` "/Game/Widgets/Dialogue/W_Dialogue.W_Dialogue_C"))
  (`UserWidget.AddToViewport` _returnvalue 0)
  (bind _asplayer (cast `/Game/Player/Player` (`GameplayStatics.GetPlayerCharacter` 0)))
  (set `/Game/Player/Player.dialogueWidget` _returnvalue _asplayer)
  (bind _asaic (cast `/Game/Blueprints/AIC` (`AIBlueprintHelperLibrary.GetAIController` self)))
  (bind _ascustom_game_instance (cast `/Game/Player/CustomGameInstance` (`GameplayStatics.GetGameInstance`)))
  (bind _dialoguetree (`/Game/Player/CustomGameInstance.dialogueTree` _ascustom_game_instance))
  (`/Game/Blueprints/AIC.StartDialogue` _asaic (select `bool` (`KismetSystemLibrary.IsValid` _dialoguetree) :`false` (`self.dialogueTree`) :`true` _dialoguetree))
  (set `/Game/Player/Player.canMove` false _asplayer)
  (set `/Game/Player/Player.isInDialogue` true _asplayer))

(event `/Game/Blueprints/Items/Parent/ObjectInterface.SetMaterial`
  (params (canSetOutline :type Boolean))
  (bind _cube (`self.Cube`))
  (if canSetOutline
    (`/Engine/EditorBlueprintResources/StandardMacros.DoOnce` false :!label _label
      (:`Completed`
        (bind _returnvalue (`AddComponent|NODE_AddStaticMeshComponent-0` :`RelativeTransform` (`SceneComponent.GetRelativeTransform` _cube)))
        (bind _output_get (set `self.outlineMesh` _returnvalue))
        (`StaticMeshComponent.SetStaticMesh` _output_get (`StaticMeshComponent.StaticMesh` _cube))
        (for _ (range (`KismetArrayLibrary.Array_Length` (`MeshComponent.GetMaterials` (`self.outlineMesh`))))
          (`PrimitiveComponent.SetMaterial` (`self.outlineMesh`) 0 "/Game/Blueprints/Items/Parent/Inst_ItemHighLight.Inst_ItemHighLight"))))
    (else
      (bind _outlinemesh (`self.outlineMesh`)
        (:`then`
          (`ActorComponent.K2_DestroyComponent` _outlinemesh)
          (goto _label :!via `Reset`))
        (:`else`)))))

(fn `Combine`
  (params (actorToUseWith :type "Actor Object Reference"))
  (returns (objectDestroyed :type Boolean))
  (return false))

(fn `UserConstructionScript`)