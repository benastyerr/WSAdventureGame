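; HintSetter is a trigger volume that sets the game's current hint when the player enters it.
; A Box overlap by the player's capsule passes a DoOnce, then writes Hint to CustomGameInstance and adds the actor to the gamemode's LevelSaveObject array.
; An Activation event sets CantSetHint, which feeds the DoOnce to block the hint.
; Combine always returns false.
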(event `/Game/Blueprints/Items/Parent/ObjectInterface.Activation`
  (set `self.cantSetHint` true))

(event `self.Box.OnComponentBeginOverlap`
  (params (OverlappedComponent :type "PrimitiveComponent Object Reference") (OtherActor :type "Actor Object Reference") (OtherComp :type "PrimitiveComponent Object Reference") (OtherBodyIndex :type Integer) (bFromSweep :type Boolean) (SweepResult :type "HitResult Structure (by ref)"))
  (bind _asplayer (cast `/Game/Player/Player` OtherActor))
  (if (== OtherComp (`Character.CapsuleComponent` _asplayer))
    (`/Engine/EditorBlueprintResources/StandardMacros.DoOnce` (`self.cantSetHint`)
      (:`Completed`
        (bind _ascustom_game_instance (cast `/Game/Player/CustomGameInstance` (`GameplayStatics.GetGameInstance`)))
        (set `/Game/Player/CustomGameInstance.hint` (`self.hint`) _ascustom_game_instance)
        (`/Game/Player/LevelSave.AddToArray` (`/Game/Player/PointAndClickGamemode.LevelSaveObject` (`/Game/Player/Player.Gamemode` _asplayer)) self)))))

(fn `Combine`
  (params (actorToUseWith :type "Actor Object Reference"))
  (returns (objectDestroyed :type Boolean))
  (return false))

(fn `UserConstructionScript`)